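; PC_MP is a multiplayer player controller that manages the local player's HUD widget.
; The ClientHostLogin event calls SetupGameHUD, which creates W_mp_hud for the local controller only, stores it and adds it to the viewport.
; ClientHostLogin then casts the game mode to MP_GM but does nothing with the result.
; EndPlay removes the stored HUD from its parent if it is still valid.
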(event `ClientHostLogin`
  (`self.SetupGameHUD`)
  (cast `/Game/Multiplayer/Blueprints/MP_GM` (`GameplayStatics.GetGameMode`)))

(event `self.ReceiveEndPlay`
  (params (EndPlayReason :type "EEndPlayReason Enum" :default "Destroyed"))
  (bind _hud (`self.HUD`))
  (`/Engine/EditorBlueprintResources/StandardMacros.IsValid` _hud
    (:`Is Valid`
      (`Widget.RemoveFromParent` _hud))))

(fn `SetupGameHUD`
  (if (`self.IsLocalPlayerController`)
    (bind _returnvalue (`|CreateWidget` "/Game/Multiplayer/Widgets/w_mp_hud.w_mp_hud_C" self))
    (bind _output_get (set `self.HUD` _returnvalue))
    (`UserWidget.AddToViewport` _output_get 0)))

(fn `UserConstructionScript`)