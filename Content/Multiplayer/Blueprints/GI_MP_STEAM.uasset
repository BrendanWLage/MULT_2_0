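; Game instance that runs the multiplayer menu flow and session hosting, joining and teardown.
; A StateTransition macro switches between main menu, server list, loading, playing and error states, hiding the outgoing widget or destroying the session when leaving play.
; Show events lazily create their widgets and set UI-only input.
; Session, network and travel failures feed DisplayError, which destroys the session and shows an error dialog.
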(event `ShowLoadScreen`
  (`self.StateTransition` "NewEnumerator6"
    (:`NewState`
      (`/Engine/EditorBlueprintResources/StandardMacros.IsValid` (`self.Loading`)
        (:`Is Valid`
          _)
        (:`Is Not Valid`
          (bind _returnvalue (`|CreateWidget` "/Game/Multiplayer/Widgets/w_loading.w_loading_C" (`GameplayStatics.GetPlayerController` 0)))
          (bind _output_get (set `self.Loading` _returnvalue))))
      (`UserWidget.AddToViewport` _output_get 0)
      (`WidgetBlueprintLibrary.SetInputMode_UIOnlyEx` null _output_get))))

(event `JoinFromServerList`
  (params (SearchResult :type "BlueprintSessionResult Structure"))
  (`self.ShowLoadScreen`)
  (`JoinSessionCallbackProxy.JoinSession` (`GameplayStatics.GetPlayerController` 0) SearchResult
    (:`OnFailure`
      (`self.DisplayError` "Failed to join Server"))))

(event `ShowServerList`
  (bind _returnvalue (`GameplayStatics.GetPlayerController` 0))
  (`self.StateTransition` "NewEnumerator4"
    (:`NewState`
      (`/Engine/EditorBlueprintResources/StandardMacros.IsValid` null
        (:`Is Valid`
          _)
        (:`Is Not Valid`
          (bind _returnvalue_2 (`|CreateWidget` "/Game/Multiplayer/Widgets/w_serverlist.w_serverlist_C" _returnvalue))
          (bind _output_get (set `self.ServerList` _returnvalue_2))))
      (`UserWidget.AddToViewport` _output_get 0)
      (`WidgetBlueprintLibrary.SetInputMode_UIOnlyEx` _returnvalue _output_get))))

(event `ShowMainMenu`
  (bind _returnvalue (`GameplayStatics.GetPlayerController` 0))
  (`self.isCurrentState` "NewEnumerator2"
    (:`True`
      (`GameplayStatics.OpenLevel` "MainMenu"))
    (:`False`
      _))
  (`self.StateTransition` "NewEnumerator1"
    (:`NewState`
      (`/Engine/EditorBlueprintResources/StandardMacros.IsValid` (`self.MainMenu`)
        (:`Is Valid`
          _)
        (:`Is Not Valid`
          (bind _returnvalue_2 (`|CreateWidget` "/Game/Multiplayer/Widgets/w_mainmenu.w_mainmenu_C" _returnvalue))
          (bind _output_get (set `self.MainMenu` _returnvalue_2))))
      (`WidgetBlueprintLibrary.SetInputMode_UIOnlyEx` _returnvalue _output_get)
      (`UserWidget.AddToViewport` _output_get 0))))

(event `HostGameEvent`
  (`self.ShowLoadScreen`)
  (`CreateSessionCallbackProxy.CreateSession` (`GameplayStatics.GetPlayerController` 0) 2 (`self.bEnableLAN`)
    (:`OnSuccess`
      (`GameplayStatics.OpenLevel` "MP_Level_1" true "listen"))
    (:`OnFailure`
      (`self.DisplayError` "Could create session"))))

(event `DestroySessCaller`
  (`DestroySessionCallbackProxy.DestroySession` (`GameplayStatics.GetPlayerController` 0)))

(event `self.HandleNetworkError`
  (params (FailureType :type "ENetworkFailure Enum" :default "NetDriverAlreadyExists") (bIsServer :type Boolean))
  (if (not bIsServer)
    (`self.DisplayError` (`self.NetCodeerrorToString` FailureType))))

(event `self.HandleTravelError`
  (params (FailureType :type "ETravelFailure Enum" :default "NoLevel"))
  (`self.DisplayError` (`self.TravelErrorToSTring` FailureType)))

(fn `BeginPlay_ShowMainMenu`
  (`self.isCurrentState` "NewEnumerator0"
    (:`True`
      (`self.ShowMainMenu`))))

(fn `HideWidget`
  (params (Widin :type "Widget Object Reference"))
  (`/Engine/EditorBlueprintResources/StandardMacros.IsValid` Widin
    (:`Is Valid`
      (`Widget.RemoveFromParent` Widin))))

(fn `NetCodeerrorToString`
  (params (InError :type "ENetworkFailure Enum"))
  (returns (ErrorOut :type String))
  (switch `ENetworkFailure` InError
    (:`NetDriverAlreadyExists`
      _)
    (:`NetDriverCreateFailure`
      _)
    (:`NetDriverListenFailure`
      _)
    (:`ConnectionLost`
      _)
    (:`ConnectionTimeout`
      (return "Timed Out"))
    (:`FailureReceived`
      _)
    (:`OutdatedClient`
      _)
    (:`OutdatedServer`
      _)
    (:`PendingConnectionFailure`
      _))
  (return "Lost Connection to host"))

(fn `StartPlayingState`
  (`self.StateTransition` "NewEnumerator2"))

(fn `TravelErrorToSTring`
  (params (InError :type "ETravelFailure Enum"))
  (returns (ErrorOut :type String))
  (return (`KismetStringLibrary.Concat_StrStr` "Error Travelling maps due to: " (`|GetEnumeratorNameAsString` InError))))