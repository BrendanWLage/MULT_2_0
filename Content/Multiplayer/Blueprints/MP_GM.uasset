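; MP_GM is a multiplayer game mode that handles player login and respawning.
; On PostLogin with authority, it numbers the player's PS_state by PlayerArray length and calls ClientHostLogin on PC_MP.
; RespawnPlayerEvent destroys the pawn, waits MinRespawnDelay, then spawns and possesses a FirstPersonCharacter at a PlayerStart.
; It picks that start by re-rolling a random index on each loop iteration, so selection is not uniform.
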(event `RespawnPlayerEvent`
  (params (PlayerController :type "PlayerController Object Reference"))
  (`self.K2_DestroyActor` (`Controller.K2_GetPawn` PlayerController))
  (`KismetSystemLibrary.Delay` (`self.MinRespawnDelay`))
  (bind _outactors (`GameplayStatics.GetAllActorsOfClass` "/Script/Engine.PlayerStart"))
  (for (_array_element _array_index) _outactors
    (if (== (`KismetMathLibrary.RandomIntegerInRange` 0 (`KismetArrayLibrary.Array_Length` _outactors)) _array_index)
      (break)))
  (bind _returnvalue (`|SpawnActorFromClass` "/Game/FirstPersonBP/Blueprints/FirstPersonCharacter.FirstPersonCharacter_C" (`self.GetTransform` _array_element) "AdjustIfPossibleButAlwaysSpawn" "OverrideRootScale"))
  (`Controller.Possess` PlayerController _returnvalue))

(event `self.K2_PostLogin`
  (params (NewPlayer :type "PlayerController Object Reference"))
  (`/Engine/EditorBlueprintResources/ActorMacros.Switch Has Authority`
    (:`Authority`
      (bind _asps_state (cast `/Game/Multiplayer/Blueprints/PS_state` (`Controller.PlayerState` NewPlayer)))
      (set `/Game/Multiplayer/Blueprints/PS_state.Player Number` (`KismetArrayLibrary.Array_Length` (`GameState.PlayerArray` (`GameplayStatics.GetGameState`))) _asps_state)
      (bind _aspc_mp (cast `/Game/Multiplayer/Blueprints/PC_MP` NewPlayer))
      (`/Game/Multiplayer/Blueprints/PC_MP.ClientHostLogin` _aspc_mp))))

(fn `UserConstructionScript`)